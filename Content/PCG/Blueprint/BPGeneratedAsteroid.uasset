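; Procedural asteroid actor assembled from six child-actor mesh pieces, each oriented by its own up vector.
; The construction script rebuilds an array of these BPGeneratedAsteroidMesh3 children, then calls SetupMesh on each with the shared size and material plus the matching up vector.
; All work happens in the construction script, with no active runtime logic.
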(event EventBeginPlay)

(event Collision|EventActorBeginOverlap
  (params (OtherActor :type Actor%20Object%20Reference)))

(event EventTick
  (params (DeltaSeconds :type Float%20%28single-precision%29)))

(fn ConstructionScript
  (bind _generated_asteroids (Variables|Default|GetGenerated%20Asteroids))
  (Utilities|Array|Clear (Variables|Default|GetGenerated%20Asteroids))
  ;[1 1 1] Add all meshes to one array
  (bind _asbpgenerated_asteroid_mesh_3 (Utilities|Casting|CastToBPGeneratedAsteroidMesh3 (Variables|/Script/Engine.ChildActorComponent|GetChildActor (Variables|Default|GetBPGeneratedAsteroidMesh3))))
  (Utilities|Array|Add (Variables|Default|GetGenerated%20Asteroids) _asbpgenerated_asteroid_mesh_3)
  (bind _asbpgenerated_asteroid_mesh_3_2 (Utilities|Casting|CastToBPGeneratedAsteroidMesh3 (Variables|/Script/Engine.ChildActorComponent|GetChildActor (Variables|Default|GetBPGeneratedAsteroidMesh4))))
  (Utilities|Array|Add (Variables|Default|GetGenerated%20Asteroids) _asbpgenerated_asteroid_mesh_3_2)
  (bind _asbpgenerated_asteroid_mesh_3_3 (Utilities|Casting|CastToBPGeneratedAsteroidMesh3 (Variables|/Script/Engine.ChildActorComponent|GetChildActor (Variables|Default|GetBPGeneratedAsteroidMesh5))))
  (Utilities|Array|Add (Variables|Default|GetGenerated%20Asteroids) _asbpgenerated_asteroid_mesh_3_3)
  (bind _asbpgenerated_asteroid_mesh_3_4 (Utilities|Casting|CastToBPGeneratedAsteroidMesh3 (Variables|/Script/Engine.ChildActorComponent|GetChildActor (Variables|Default|GetBPGeneratedAsteroidMesh6))))
  (Utilities|Array|Add (Variables|Default|GetGenerated%20Asteroids) _asbpgenerated_asteroid_mesh_3_4)
  (bind _asbpgenerated_asteroid_mesh_3_5 (Utilities|Casting|CastToBPGeneratedAsteroidMesh3 (Variables|/Script/Engine.ChildActorComponent|GetChildActor (Variables|Default|GetBPGeneratedAsteroidMesh7))))
  (Utilities|Array|Add (Variables|Default|GetGenerated%20Asteroids) _asbpgenerated_asteroid_mesh_3_5)
  (bind _asbpgenerated_asteroid_mesh_3_6 (Utilities|Casting|CastToBPGeneratedAsteroidMesh3 (Variables|/Script/Engine.ChildActorComponent|GetChildActor (Variables|Default|GetBPGeneratedAsteroidMesh8))))
  (Utilities|Array|Add _generated_asteroids _asbpgenerated_asteroid_mesh_3_6)
  ;[1 1 1] Setup Mesh for each meshes and apply texture
  (for (_array_element _array_index) _generated_asteroids
    (Class|GeneratedAsteroidMesh3|SetupMesh _array_element (Variables|Default|GetSize) (Utilities|Array|Get(acopy) (Variables|Default|GetUpVectors) _array_index) "/Game/PCG/AsteroidMaterial.AsteroidMaterial")))